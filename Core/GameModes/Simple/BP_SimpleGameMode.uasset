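; BP_SimpleGameMode is a turn-based battle game mode where participants take turns based on the order they were added.
; StartBattle extends the parent by setting each participant's Counter to its array index.
; GetNextParticipant runs the parent's victory check, selects the participant at the current index and refreshes the turn order widget.
; SpawnRandomEnemies spawns a random number of BP_Participant actors in an evenly spaced row.
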(event `self.StartBattle`
  ;[1 1 1] Start Battle Override - Set counter to order added
  (`parent.StartBattle`)
  (for (_array_element _array_index) (`self.Participants`)
    (set `/Game/TurnBasedBattleSystems/Core/Characters/BP_Participant.Counter` _array_index _array_element)))

(fn `GetNextParticipant`
  (returns (NextParticipant :type "/Game/TurnBasedBattleSystems/Core/Characters/BP_Participant Object Reference"))
  (locals (NextParticipantFromIndex :type "/Game/TurnBasedBattleSystems/Core/Characters/BP_Participant Object Reference"))
  ;[1 1 1] Parent call for victory check
  (`parent.GetNextParticipant`)
  ;[1 1 1] Get next participant from the current index and store the value
  (bind _nextparticipant (`self.GetParticipantFromCurrentIndex` (`self.Participants`)))
  (set `local.NextParticipantFromIndex` _nextparticipant)
  ;[1 1 1] Update the turn order
  (`self.UpdateTurnOrderWidget` (`self.Participants`))
  ;[1 1 1] Return the next participant
  (return (`local.NextParticipantFromIndex`)))

(fn `SpawnRandomEnemies`
  (locals (MaxNumberOfEneimes :type Integer :default 3) (VerticalOffset :type "Float (double-precision)" :default -200.0) (GapBetweenEnemies :type "Float (double-precision)" :default 150.0) (`Current Index` :type Integer))
  (for _index (range (+ (+ (`KismetMathLibrary.RandomInteger` (`local.MaxNumberOfEneimes`)) 1) 1))
    (bind _output_get (set `local.Current Index` _index))
    (`|SpawnActorFromClass` "/Game/TurnBasedBattleSystems/Core/Characters/BP_Participant.BP_Participant_C" (`KismetMathLibrary.MakeTransform` (`KismetMathLibrary.MakeVector` (+ (* _output_get (`local.VerticalOffset`)) (`local.GapBetweenEnemies`)) -350.0 88.0) (struct :`Yaw` 90.0)) "Undefined" "OverrideRootScale" null 0 0.0 50.0 25.0 (`KismetStringLibrary.Conv_IntToString` (`local.Current Index`)) 0 null)))

(fn `UserConstructionScript`
  (`parent.UserConstructionScript`))